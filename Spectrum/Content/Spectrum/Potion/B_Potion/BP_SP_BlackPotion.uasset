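; BP_SP_BlackPotion is a throwable potion that explodes on hit, dealing full radial damage around the impact point.
; Throw runs once, detaching the actor, launching it through ProjectileMovement and switching the sphere to black-item collision, then tweens the grenade mesh to a random rotation.
; Hit triggers the ExplosiveComponent, applies the damage, hides the mesh and sets a short lifespan for cleanup.
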(event `self.ReceiveBeginPlay`)

(event `Throw`
  (params (Velocity :type "Vector Structure"))
  (bind _projectilemovement (`self.ProjectileMovement`))
  (`/Engine/EditorBlueprintResources/StandardMacros.DoOnce` false
    (:`Completed`
      (`|ExecutionSequence`
        (:`then_0`
          (`self.K2_DetachFromActor` "KeepWorld" "KeepWorld" "KeepWorld")
          (set `MovementComponent.Velocity` Velocity _projectilemovement)
          (`ActorComponent.Activate` _projectilemovement false)
          (`PrimitiveComponent.SetCollisionProfileName` (`self.Sphere`) "BlackItemCollision" true))
        (:`then_1`
          (`KismetSystemLibrary.MoveComponentTo` (`self.SM_Grenade`) (0.0 0.0 0.0) (`KismetMathLibrary.RandomRotator` false) false false 0.5))))))

(event `self.ReceiveHit`
  (params (MyComp :type "PrimitiveComponent Object Reference") (Other :type "Actor Object Reference") (OtherComp :type "PrimitiveComponent Object Reference") (bSelfMoved :type Boolean) (HitLocation :type "Vector Structure") (HitNormal :type "Vector Structure") (NormalImpulse :type "Vector Structure") (Hit :type "HitResult Structure (by ref)"))
  (`/Game/Spectrum/BluePrint/BP_EC.Explode` (`self.ExplosiveComponent`))
  (`GameplayStatics.ApplyRadialDamage` :`BaseDamage` 100.0 :`Origin` HitLocation :`DamageRadius` 100.0 :`DamageCauser` self :`InstigatedByController` null :`bDoFullDamage` true :`DamagePreventionChannel` "ECC_Pawn")
  (`SceneComponent.SetHiddenInGame` (`self.SM_Grenade`) true false)
  (`self.SetLifeSpan` 1.0))

(fn `UserConstructionScript`)