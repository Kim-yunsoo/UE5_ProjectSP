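; BP_SPCharacterMan is a Spectrum character Blueprint whose events, construction script and grenade path event are all empty in this graph.
; Disconnected leftover logic compares control-rotation yaw against a stored value to set turn-left/right flags, clearing them while moving.
; Other unwired fragments create a WB_TargetUI widget and print debug text, so none of this logic runs.
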(event `self.ReceiveTick`
  (params (DeltaSeconds :type "Float (single-precision)")))

(event `self.ReceiveBeginPlay`)

(event `InputAxis|Turn Right / Left Mouse`
  (params (AxisValue :type "Float (single-precision)")))

(event `ShowProjectilePath`)

(fn `UserConstructionScript`)