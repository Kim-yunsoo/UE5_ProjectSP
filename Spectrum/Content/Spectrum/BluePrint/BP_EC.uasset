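; BP_EC is a component that makes its owning actor explode once, damaging nearby actors.
; Explode spawns an explosion particle at the owner, then runs a debug-drawn sphere overlap for WorldDynamic objects.
; Hit actors join a unique array and receive OnExplosionHitMessage with source and damage; the message loop is nested inside the hit loop, so actors can be messaged repeatedly.
; A sound-playing branch is left unconnected.
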(event `self.ReceiveTick`
  (params (DeltaSeconds :type "Float (single-precision)")))

(event `Explode`
  (bind _returnvalue (`SceneComponent.K2_GetComponentLocation` (`Actor.RootComponent` (`self.GetOwner`))))
  (`/Engine/EditorBlueprintResources/StandardMacros.DoOnce` false
    (:`Completed`
      (`GameplayStatics.SpawnEmitterAtLocation` "/Game/Box/MagicStaff/Demo/Particles/P_Explosion.P_Explosion" (`Actor.K2_GetActorLocation` (`self.GetOwner`)))
      (bind (_outhits _returnvalue_2) (`KismetSystemLibrary.SphereTraceMultiForObjects` :`Start` _returnvalue :`End` _returnvalue :`Radius` 100.0 :`ObjectTypes` (`|MakeArray` "ObjectTypeQuery2" :!type "EObjectTypeQuery Enum") :`DrawDebugType` "ForDuration"))
      (if _returnvalue_2
        (for _array_element _outhits
          (`KismetArrayLibrary.Array_AddUnique` (`self.Nearby Actors`) (`.HitActor` (`GameplayStatics.BreakHitResult` _array_element)))
          (if (> (`KismetArrayLibrary.Array_Length` (`self.Nearby Actors`)) 0)
            (for _array_element_2 (`self.Nearby Actors`)
              (message `/Game/Spectrum/BluePrint/interface/BPI_Damageable.On Explosion Hit` _array_element_2 (`self.GetOwner`) 200.0))))))))