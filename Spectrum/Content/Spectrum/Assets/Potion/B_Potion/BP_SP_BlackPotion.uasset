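; BP_SP_BlackPotion is a throwable black potion actor driven by a projectile movement component.
; Its Throw event fires only once, detaching the potion with its world transform kept, applying the given velocity and activating projectile movement.
; It then switches the sphere's collision to the BlackItemCollision profile and rotates the grenade mesh toward a random orientation over half a second.
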(event `self.ReceiveBeginPlay`)

(event `Throw`
  (params (Velocity :type "Vector Structure"))
  (bind _projectilemovement (`self.ProjectileMovement`))
  (`/Engine/EditorBlueprintResources/StandardMacros.DoOnce` false
    (:`Completed`
      (`|ExecutionSequence`
        (:`then_0`
          (`self.K2_DetachFromActor` "KeepWorld" "KeepWorld" "KeepWorld")
          (set `MovementComponent.Velocity` Velocity _projectilemovement)
          (`ActorComponent.Activate` _projectilemovement false)
          (`PrimitiveComponent.SetCollisionProfileName` (`self.Sphere`) "BlackItemCollision" true))
        (:`then_1`
          (`KismetSystemLibrary.MoveComponentTo` (`self.SM_Grenade`) (0.0 0.0 0.0) (`KismetMathLibrary.RandomRotator` false) false false 0.5))))))

(fn `UserConstructionScript`)