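; BP_Book is a book actor that tints its mesh green at runtime.
; BeginPlay creates a dynamic material instance on ObjectMesh, and Tick sets its Base Color Tint to green once when the IsOnce flag is true, then clears the flag.
; Disconnected leftover nodes for physics, geometry collection impulse, collision changes and destruction never run.
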(event `self.ReceiveBeginPlay`
  (bind _returnvalue (`PrimitiveComponent.CreateDynamicMaterialInstance` (`self.ObjectMesh`) 0 null "None"))
  (set `self.Dynamic Material` _returnvalue))

(event `self.ReceiveTick`
  (params (DeltaSeconds :type "Float (single-precision)"))
  (if (`self.IsOnce`)
    (if true
      (set `self.IsOnce` false)
      (`MaterialInstanceDynamic.SetVectorParameterValue` (`self.Dynamic Material`) "Base Color Tint" (`self.GreenLinearColor`)))))

(fn `UserConstructionScript`)