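; BP_Box is a destructible box prop that breaks on receiving any damage.
; On AnyDamage it prints its name and the damage amount, hides its static mesh and adds a Geometry Collection component at runtime in its place.
; It then sets a short lifespan so the actor cleans itself up.
; There is no health check, and the RadialDamage handler is empty.
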(event `self.ReceiveTick`
  (params (DeltaSeconds :type "Float (single-precision)")))

(event `self.ReceiveAnyDamage`
  (params (Damage :type "Float (single-precision)") (DamageType :type "DamageType Object Reference") (InstigatedBy :type "Controller Object Reference") (DamageCauser :type "Actor Object Reference"))
  (`KismetSystemLibrary.PrintString` (`KismetStringLibrary.Concat_StrStr` (`KismetSystemLibrary.GetDisplayName` self) ":    " (`KismetStringLibrary.Conv_DoubleToString` Damage)))
  (`SceneComponent.SetHiddenInGame` (`self.StaticMeshComponent`) true false)
  (`AddComponent|NODE_AddGeometryCollectionComponent-0`)
  (`self.SetLifeSpan` 5.0))

(event `self.ReceiveRadialDamage`
  (params (DamageReceived :type "Float (single-precision)") (DamageType :type "DamageType Object Reference") (Origin :type "Vector Structure") (HitInfo :type "HitResult Structure (by ref)") (InstigatedBy :type "Controller Object Reference") (DamageCauser :type "Actor Object Reference")))

(fn `UserConstructionScript`)